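; Battery pickup variant that shows electric arcs between itself and the player when targeted or collected.
; Every tick, it creates a white beam while it is in the ThirdPersonCharacter's TargetedActors, aims it at the player's spine socket, and destroys it otherwise.
; On collection, a red arc re-aims at that socket through a repeating 0.1-second delay loop, while the parent's collect logic runs after a half-second delay.
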(event `self.ReceiveTick`
  (params (DeltaSeconds :type "Float (single-precision)"))
  (`self.TargetingBeam`))

(event `self.OnCollected`
  (bind _returnvalue (`GameplayStatics.SpawnEmitterAttached` "/Game/ExampleContent/Effects/ParticleSystems/P_electricity_arc_red.P_electricity_arc_red" (`self.PickupMesh`)))
  (`ParticleSystemComponent.SetBeamTargetPoint` _returnvalue 0 (`SceneComponent.GetSocketLocation` (`Character.Mesh` (`GameplayStatics.GetPlayerCharacter` 0)) "spine_03") 0 :!label _label)
  (`|ExecutionSequence`
    (:`then_0`
      (`KismetSystemLibrary.Delay` 0.5)
      (`parent.OnCollected`))
    (:`then_1`
      (`KismetSystemLibrary.Delay` 0.1)
      (goto _label))))

(fn `TargetingBeam`
  (bind _targetingparticlesys (`self.TargetingParticleSys`))
  (bind _returnvalue (`KismetSystemLibrary.IsValid` _targetingparticlesys))
  (bind _asthird_person_character (cast `/Game/MyContent/Blueprints/ThirdPersonCharacter` (`GameplayStatics.GetPlayerCharacter` 0)))
  (if (`KismetArrayLibrary.Array_Contains` (`MyProjectTestCharacter.TargetedActors` _asthird_person_character) self)
    (if (not _returnvalue)
      (bind _returnvalue_2 (`GameplayStatics.SpawnEmitterAttached` "/Game/ExampleContent/Effects/ParticleSystems/P_electricity_arc_white.P_electricity_arc_white" (`self.PickupMesh`) "None" (0.0 0.0 0.0) (struct) (1.0 1.0 1.0) "KeepRelativeOffset" false))
      (bind _output_get (set `self.TargetingParticleSys` _returnvalue_2)))
    (`ParticleSystemComponent.SetBeamTargetPoint` _targetingparticlesys 0 (`SceneComponent.GetSocketLocation` (`Character.Mesh` (`GameplayStatics.GetPlayerCharacter` 0)) "spine_03") 0)
    (`ParticleSystemComponent.SetBeamTargetPoint` _output_get 0 (`SceneComponent.GetSocketLocation` (`Character.Mesh` (`GameplayStatics.GetPlayerCharacter` 0)) "spine_03") 0) ; set beam target to player
    (elif _returnvalue
      (`ActorComponent.K2_DestroyComponent` _targetingparticlesys))))

(fn `UserConstructionScript`)