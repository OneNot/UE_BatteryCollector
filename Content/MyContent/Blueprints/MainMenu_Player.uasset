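; MainMenu_Player is a pawn, apparently for the main menu, that wanders randomly around the navigable area by itself.
; BeginPlay picks a random navigable point within a large radius of the mesh and sends the controller there with SimpleMoveToLocation.
; Tick measures the distance to that target, picking a new one when close and otherwise reissuing the move every frame.
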(event `self.ReceiveBeginPlay`
  (bind (_randomlocation _returnvalue) (`NavigationSystemV1.K2_GetRandomLocationInNavigableRadius` (`SceneComponent.K2_GetComponentLocation` (`self.Mesh`)) 9000.0 null null))
  (if _returnvalue :!label _label
    (bind _output_get (set `self.Target` _randomlocation))
    (`AIBlueprintHelperLibrary.SimpleMoveToLocation` (`self.GetController`) _output_get :!label _label_2)))

(event `self.ReceiveTick`
  (params (DeltaSeconds :type "Float (single-precision)"))
  (bind _returnvalue (`KismetMathLibrary.Vector_Distance` (`SceneComponent.K2_GetComponentLocation` (`self.Mesh`)) (`self.Target`)))
  (`KismetSystemLibrary.PrintString` (`KismetStringLibrary.Conv_DoubleToString` _returnvalue) false false)
  (if (<= _returnvalue 100.0)
    (goto _label)
    (else
      (goto _label_2))))

(fn `UserConstructionScript`)