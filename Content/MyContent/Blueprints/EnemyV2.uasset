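; EnemyV2 is an enemy that chases the player and drains their power with a red electric arc.
; Each Tick it moves toward the player pawn, stopping within StopDistance, and logs the current distance.
; Within AttackRange it spawns an attached beam emitter if needed, aims it at the player's spine socket, and reduces ThirdPersonCharacter power by delta-scaled Damage.
; Outside that range it destroys the emitter.
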(event `self.ReceiveTick`
  (params (DeltaSeconds :type "Float (single-precision)"))
  (bind _returnvalue (`self.GetController`))
  (bind _returnvalue_2 (`GameplayStatics.GetPlayerPawn` 0))
  (bind _particlesystem (`self.particleSystem`))
  (bind _returnvalue_3 (`KismetSystemLibrary.IsValid` _particlesystem))
  (bind _returnvalue_4 (`KismetMathLibrary.Vector_Distance` (`SceneComponent.K2_GetComponentLocation` (`self.Mesh`)) (`self.K2_GetActorLocation` _returnvalue_2)))
  (if (> _returnvalue_4 (`self.StopDistance`))
    (`AIBlueprintHelperLibrary.SimpleMoveToActor` _returnvalue _returnvalue_2)
    (else
      (`Controller.StopMovement` _returnvalue)))
  (`KismetSystemLibrary.PrintString` (`KismetStringLibrary.Conv_DoubleToString` _returnvalue_4) false)
  (if (<= _returnvalue_4 (`self.AttackRange`))
    (if (not _returnvalue_3)
      (bind _returnvalue_5 (`GameplayStatics.SpawnEmitterAttached` "/Game/ExampleContent/Effects/ParticleSystems/P_electricity_arc_red.P_electricity_arc_red" (`self.Mesh`) "None" (0.0 0.0 0.0) (struct) (1.0 1.0 1.0) "KeepRelativeOffset" false))
      (set `self.particleSystem` _returnvalue_5))
    (`ParticleSystemComponent.SetBeamTargetPoint` _particlesystem 0 (`SceneComponent.GetSocketLocation` (`Character.Mesh` (`GameplayStatics.GetPlayerCharacter` 0)) "spine_03") 0)
    (bind _asthird_person_character (cast `/Game/MyContent/Blueprints/ThirdPersonCharacter` _returnvalue_2))
    (`MyProjectTestCharacter.UpdatePower` _asthird_person_character (* (`self.Damage`) DeltaSeconds -1.0))
    (elif _returnvalue_3
      (`ActorComponent.K2_DestroyComponent` _particlesystem))))

(fn `UserConstructionScript`)