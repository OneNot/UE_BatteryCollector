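; MainMenuEnemyV2 is an enemy that follows a target character and zaps it with a red electric beam, with no damage logic.
; Every Tick it moves toward the target via SimpleMoveToLocation until within StopDistance, then stops.
; Within AttackRange it spawns an arc emitter on its spine socket once and updates the beam end to the target's spine each frame.
; Out of range, it destroys the emitter.
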(event `self.ReceiveTick`
  (params (DeltaSeconds :type "Float (single-precision)"))
  (bind _returnvalue (`self.GetController`))
  (bind _targetchar (`self.TargetChar`))
  (bind _particlesystem (`self.particleSystem`))
  (bind _returnvalue_2 (`self.K2_GetActorLocation` _targetchar))
  (bind _returnvalue_3 (`KismetSystemLibrary.IsValid` _particlesystem))
  (bind _returnvalue_4 (`KismetMathLibrary.Vector_Distance` (`SceneComponent.K2_GetComponentLocation` (`self.Mesh`)) _returnvalue_2))
  ;[1 1 1] Move Enemy closer to and stop at X distance from player
  (if (> _returnvalue_4 (`self.StopDistance`))
    (`AIBlueprintHelperLibrary.SimpleMoveToLocation` _returnvalue _returnvalue_2)
    (else
      (`Controller.StopMovement` _returnvalue)))
  (`KismetSystemLibrary.PrintString` (`KismetStringLibrary.Conv_DoubleToString` _returnvalue_4) false false)
  ;[1 1 1] Shoot Negative power beam at player if close enough
  (if (<= _returnvalue_4 (`self.AttackRange`))
    (if (not _returnvalue_3)
      (bind _returnvalue_5 (`GameplayStatics.SpawnEmitterAttached` "/Game/ExampleContent/Effects/ParticleSystems/P_electricity_arc_red.P_electricity_arc_red" (`self.Mesh`) "spine_03" (0.0 0.0 0.0) (struct) (1.0 1.0 1.0) "KeepRelativeOffset" false))
      (set `self.particleSystem` _returnvalue_5))
    (`ParticleSystemComponent.SetBeamTargetPoint` _particlesystem 0 (`SceneComponent.GetSocketLocation` (`Actor.RootComponent` _targetchar) "spine_03") 0)
    (elif _returnvalue_3
      (`ActorComponent.K2_DestroyComponent` _particlesystem))))

(fn `UserConstructionScript`)